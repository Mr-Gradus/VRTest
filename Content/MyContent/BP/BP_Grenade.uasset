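; BP_Grenade is a grenade Blueprint that simulates a timed fuse using printed messages only.
; TriggerReleased passes through a DoOnce to start a looping one-second timer, so the fuse starts only once.
; Each tick of the timer runs through a DoN counter that prints beeps, then a boom on the final count.
; The timer is never cleared; DoN silences further ticks, and no damage or effects are implemented.
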(event `/Game/VRTemplate/Blueprints/VRInteractionBPI.TriggerReleased`
  (`/Engine/EditorBlueprintResources/StandardMacros.DoOnce` false
    (:`Completed`
      (`KismetSystemLibrary.K2_SetTimerDelegate` (delegate `Timer`) 1.0 true))))

(event `Timer`
  (bind _counter (`/Engine/EditorBlueprintResources/StandardMacros.Do N` 5)
    (:`Exit`
      (if (== _counter 5)
        (`KismetSystemLibrary.PrintString` "***BOOM***" true true (struct :`R` 0.770833 :`G` 0.057058 :`A` 1.0))
        (else
          (`KismetSystemLibrary.PrintString` "*BEEP*"))))))

(fn `UserConstructionScript`
  (`parent.UserConstructionScript`))