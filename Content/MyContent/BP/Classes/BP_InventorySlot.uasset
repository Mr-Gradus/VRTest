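; BP_InventorySlot is an inventory slot actor that tracks the item inside its sphere, apparently for motion-controller (VR) grabbing.
; Sphere overlaps store the latest BP_InventoryItemClass as ItemInSlot and clear it when that item exits.
; Put calls TryGrab on the item's GrabComponent with MotionController, then sets the slot's own location to its current one.
; An unwired "simple method" variant, which moves the item to the slot, never runs.
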(event `self.Sphere.OnComponentBeginOverlap`
  (params (OverlappedComponent :type "PrimitiveComponent Object Reference") (OtherActor :type "Actor Object Reference") (OtherComp :type "PrimitiveComponent Object Reference") (OtherBodyIndex :type Integer) (bFromSweep :type Boolean) (SweepResult :type "HitResult Structure (by ref)"))
  ;[1 1 1] Better method
  (bind _asbp_inventory_item_class (cast `/Game/MyContent/BP/Classes/BP_InventoryItemClass` OtherActor))
  (set `self.ItemInSlot` _asbp_inventory_item_class))

(event `self.Sphere.OnComponentEndOverlap`
  (params (OverlappedComponent :type "PrimitiveComponent Object Reference") (OtherActor :type "Actor Object Reference") (OtherComp :type "PrimitiveComponent Object Reference") (OtherBodyIndex :type Integer))
  ;[1 1 1] Better method
  (bind _asbp_inventory_item_class (cast `/Game/MyContent/BP/Classes/BP_InventoryItemClass` OtherActor))
  (if (== _asbp_inventory_item_class (`self.ItemInSlot`))
    (set `self.ItemInSlot` null)))

(event `Put`
  ;[1 1 1] Better method
  (`/Game/VRTemplate/Blueprints/GrabComponent.TryGrab` (`/Game/MyContent/BP/Classes/BP_Interaction_Class.GrabComponent` (`self.ItemInSlot`)) (`self.MotionController`))
  (`self.K2_SetActorLocation` (`self.K2_GetActorLocation`)))

(fn `UserConstructionScript`)